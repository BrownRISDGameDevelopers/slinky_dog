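; Player controller for the SlinkyDog two-player prototype, driving both characters from a single controller.
; On BeginPlay it finds the first BP_Proto_TwoPlayer1 and BP_Proto_TwoPlayer2 actors in the level and adds the IMC_Controls mapping context.
; Separate Enhanced Input jump and move actions for each player forward start, release, horizontal movement and stop calls to the matching actor.
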(event Input|EnhancedActionEvents|EnhancedInputActionIA_Jump1
  (params (ActionValue :type Boolean) (ElapsedSeconds :type Float%20%28double-precision%29) (TriggeredSeconds :type Float%20%28double-precision%29) (InputAction :type Input%20Action%20Object%20Reference :default "/Game/SlinkyDog/proto_twoplayer/Proto_TwoPlayerActions/IA_Jump1.IA_Jump1"))
  (bind _player1 (Variables|Default|GetPlayer1))
  (:Started
    (Default|Jump1Started _player1))
  (:Completed
    (Default|Jump1Completed _player1)))

(event Input|EnhancedActionEvents|EnhancedInputActionIA_Move1
  (params (ActionValue :type Vector%202D%20Structure) (ElapsedSeconds :type Float%20%28double-precision%29) (TriggeredSeconds :type Float%20%28double-precision%29) (InputAction :type Input%20Action%20Object%20Reference :default "/Game/SlinkyDog/proto_twoplayer/Proto_TwoPlayerActions/IA_Move1.IA_Move1"))
  (:Triggered
    (Default|Move1 (Variables|Default|GetPlayer1) (.x ActionValue)))
  (:Completed
    (Default|Stop (Variables|Default|GetPlayer1))))

(event Input|EnhancedActionEvents|EnhancedInputActionIA_Jump2
  (params (ActionValue :type Boolean) (ElapsedSeconds :type Float%20%28double-precision%29) (TriggeredSeconds :type Float%20%28double-precision%29) (InputAction :type Input%20Action%20Object%20Reference :default "/Game/SlinkyDog/proto_twoplayer/Proto_TwoPlayerActions/IA_Jump2.IA_Jump2"))
  (bind _player2 (Variables|Default|GetPlayer2))
  (:Started
    (Default|Jump2Started _player2))
  (:Completed
    (Default|Jump2Completed _player2)))

(event Input|EnhancedActionEvents|EnhancedInputActionIA_Move2
  (params (ActionValue :type Vector%202D%20Structure) (ElapsedSeconds :type Float%20%28double-precision%29) (TriggeredSeconds :type Float%20%28double-precision%29) (InputAction :type Input%20Action%20Object%20Reference :default "/Game/SlinkyDog/proto_twoplayer/Proto_TwoPlayerActions/IA_Move2.IA_Move2"))
  (:Triggered
    (Default|Move2 (Variables|Default|GetPlayer2) (.x ActionValue)))
  (:Completed
    (Default|Stop (Variables|Default|GetPlayer2))))

(event EventBeginPlay
  (bind _outactors (Actor|GetAllActorsOfClass "/Game/SlinkyDog/proto_twoplayer/BP_Proto_TwoPlayer1.BP_Proto_TwoPlayer1_C"))
  (Variables|Default|SetPlayer1 (Utilities|Array|Get(acopy) _outactors))
  (bind _outactors_2 (Actor|GetAllActorsOfClass "/Game/SlinkyDog/proto_twoplayer/BP_Proto_TwoPlayer2.BP_Proto_TwoPlayer2_C"))
  (Variables|Default|SetPlayer2 (Utilities|Array|Get(acopy) _outactors_2))
  (Input|AddMappingContext (PlayerController|LocalPlayerSubsystems|GetEnhancedInputLocalPlayerSubsystem) "/Game/SlinkyDog/proto_twoplayer/IMC_Controls.IMC_Controls" 0 "(bIgnoreAllPressedKeysUntilRelease=True,bForceImmediately=False,bNotifyUserSettings=False)"))

(fn ConstructionScript)